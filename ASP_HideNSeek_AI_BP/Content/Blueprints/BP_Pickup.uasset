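; BP_Pickup is a rotating, hovering time pickup that adds 15 seconds to the ThirdPersonGameMode timer.
; Overlap shows a "Press E to Pickup" widget and enables input, and leaving removes both.
; Interact spawns a +15 widget, destroys the actor and updates the game mode's seconds, carrying overflow into minutes.
; Tick drives frame-rate-independent yaw spin, while a BeginPlay timeline adds Z offsets for the hover.
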(event Custom|+15TimerAddon
  ;[1 1 1] Custom Event for creating the +15 seconds fade widget
  (bind _returnvalue (UserInterface|CreateWidget "/Game/Blueprints/User_Interface/InGame_UI/+15SecondsTimerAddOn.+15SecondsTimerAddOn_C"))
  (UserInterface|Viewport|AddtoViewport _returnvalue 0))

(event Collision|EventActorEndOverlap
  (params (OtherActor :type Actor%20Object%20Reference))
  ;[1 1 1] On end overlap, remove the widget (that was placed onscreen above) and disable input for within this BP
  (Widget|RemovefromParent (stale Collision|EventActorBeginOverlap _returnvalue))
  (Input|DisableInput (Game|GetPlayerController 0)))

(event Collision|EventActorBeginOverlap
  (params (OtherActor :type Actor%20Object%20Reference))
  ;[1 1 1] On overlap, put the widget for "Press E to Pickup" on screen and enable input (so player can press E within this BP)
  (bind _returnvalue (UserInterface|CreateWidget "/Game/Blueprints/User_Interface/InGame_UI/Pickup.Pickup_C"))
  (UserInterface|Viewport|AddtoViewport _returnvalue 0)
  (Input|EnableInput (Game|GetPlayerController 0)))

(event EventBeginPlay
  (bind _returnvalue (Transformation|GetActorLocation))
  ;[1 1 1] On BeginPlay, make the pickup hover up and down by using the timeline created and manipulating the pickups Z-Axis with the timeline
  (bind _hoverupanddown (Timeline|HoverUpAndDown PlayFromStart)
    (:Update
      (Transformation|SetActorLocation (Math|Vector|MakeVector (.x _returnvalue) (.y _returnvalue) (+ (.z _returnvalue) _hoverupanddown)) false false))))

(event EventTick
  (params (DeltaSeconds :type Float%20%28single-precision%29))
  ;[1 1 1] Make the pickups rotate. Event Tick to do the rotation every tick based on the delta seconds. Z axis rotated by the set rotation value (150). Multiply value by delta seconds and set this as the delta rotation
  (Transformation|AddActorLocalRotation (* (Math|Rotator|MakeRotator 0.0 0.0 (Variables|Default|Getfl_RotateValue)) DeltaSeconds) false false)
  (Transformation|AddActorLocalOffset "0, 0, 0" false false))

(event Input|ActionEvents|InputActionInteract
  (params (Key :type Key%20Structure))
  (bind _returnvalue (Game|GetGameMode))
  ;[1 1 1] Check if the player presses the interact button, destroy the actor, get the current amount of seconds, +15 onto this, then check the amount of seconds, if >=60: +1 to minutes and -60 from seconds
  (:Pressed
    (CallFunction|+15TimerAddon)
    (Actor|DestroyActor)
    (bind _asthird_person_game_mode (Utilities|Casting|CastToThirdPersonGameMode _returnvalue))
    (Variables|/Game/Blueprints/ThirdPersonGameMode.ThirdPersonGameMode_C|Seti_Seconds _asthird_person_game_mode (+ (Variables|/Game/Blueprints/ThirdPersonGameMode.ThirdPersonGameMode_C|Geti_Seconds _asthird_person_game_mode) 15))
    (bind _asthird_person_game_mode_2 (Utilities|Casting|CastToThirdPersonGameMode _returnvalue))
    (if (>= (Variables|/Game/Blueprints/ThirdPersonGameMode.ThirdPersonGameMode_C|Geti_Seconds _asthird_person_game_mode_2) 60)
      (Variables|/Game/Blueprints/ThirdPersonGameMode.ThirdPersonGameMode_C|Seti_Minutes _asthird_person_game_mode_2 (+ (Variables|/Game/Blueprints/ThirdPersonGameMode.ThirdPersonGameMode_C|Geti_Minutes _asthird_person_game_mode_2) 1))
      (Variables|/Game/Blueprints/ThirdPersonGameMode.ThirdPersonGameMode_C|Seti_Seconds _asthird_person_game_mode_2 (- (Variables|/Game/Blueprints/ThirdPersonGameMode.ThirdPersonGameMode_C|Geti_Seconds _asthird_person_game_mode_2) 60)))))

(fn ConstructionScript)